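; Card hand actor that holds card values in a Contents array and displays them as a row of BP_StandardCard actors.
; Adding a card only inserts the value into Contents, while a separate collection visuals event rebuilds the display from that data.
; Each rebuild destroys the old card actors and spawns non-replicated ones in HAND status, evenly spaced along Y from the hand's location, which is set to OriginLocation on start.
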(event Custom|AddCardToHand
  (params (Value :type Integer) (Location :type Integer))
  ;[1 1 1] Handle data
  (Utilities|Array|Insert (Variables|Default|GetContents) Value Location))

(event Custom|Update-Hand-Visuals
  (bind _contents (Variables|Default|GetContents))
  ;[1 1 1] UpdateVisuals
  (CallFunction|EmptyCards)
  (for (_ _array_index) _contents
    (if (Utilities|Array|IsValidIndex _contents _array_index)
      (bind _returnvalue (Game|SpawnActorfromClass "/Game/Blueprint/Cards/BP_StandardCard.BP_StandardCard_C" (Math|Transform|MakeTransform (+ (Transformation|GetActorLocation) (* (Math|Vector|MakeVector 0.0 5e+01 0.0) _array_index)) "-90.000000,0.000000,0.000000") "Undefined" "MultiplyWithRoot" 0 0))
      (Variables|/Script/ICAN_Card_Game.Card|SetStatus _returnvalue "IN_HAND")
      (Networking|SetReplicates _returnvalue false)
      (Utilities|Array|Insert (Variables|Default|GetCards) _returnvalue))))

(event Custom|DebugCards)

(event EventOnStart
  (Transformation|SetActorLocation (Variables|Default|GetOriginLocation) false false))

(event EventUpdateCollectionVisualstoMatchCollectionData
  (params (Collection :type Card%20Collection%20Object%20Reference))
  ;[1 1 1] UpdateVisuals
  (CallFunction|Update-Hand-Visuals)
  (CallFunction|DebugCards))

(event EventAddCardBP
  (params (Value :type Integer) (CollectionLocationToPutAt :type Integer))
  ;[1 1 1] Handle data
  (CallFunction|AddCardtoHand Value CollectionLocationToPutAt))

(fn ConstructionScript)

(fn EmptyCards
  (bind _cards (Variables|Default|GetCards))
  (for _array_element _cards
    (Utilities|IsValid _array_element
      (:Is%20Valid
        (Actor|DestroyActor _array_element))))
  (Utilities|Array|Clear _cards))