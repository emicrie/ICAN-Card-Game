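; BP_Rules_ThreeOfAKindWord is a card scoring rule that detects three of a kind by card placement.
; Its validation function counts the valid cards in the given set by their CardDataComp placement: Amplification, Body or Flavor.
; The rule passes only when one of those tallies equals exactly three, so a count of four or more in a placement does not qualify by itself.
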(fn BValidateRule
  (params (Cards :type Array%20of%20Card%20Object%20References))
  (Variables|Default|SetAmplification 0)
  (Variables|Default|SetBody 0)
  (Variables|Default|SetFlavor 0)
  (for _array_element Cards
    (Utilities|IsValid _array_element
      (:Is%20Valid
        (Utilities|FlowControl|Sequence
          (:then_0
            (if (Utilities|Enum|Equal(Enum) (Variables|/Script/ICAN_Card_Game.CardData|GetPlacement (Variables|/Script/ICAN_Card_Game.Card|GetCardDataComp _array_element)) "AMPLIFICATION")
              (bind _result (Math|Integer|IncrementInt (Variables|Default|GetAmplification))
                (:%20%20
                  (Variables|Default|SetAmplification _result)))))
          (:then_1
            (if (Utilities|Enum|Equal(Enum) (Variables|/Script/ICAN_Card_Game.CardData|GetPlacement (Variables|/Script/ICAN_Card_Game.Card|GetCardDataComp _array_element)) "BODY")
              (bind _result_2 (Math|Integer|IncrementInt (Variables|Default|GetBody))
                (:%20%20
                  (Variables|Default|SetBody _result_2)))))
          (:then_2
            (if (Utilities|Enum|Equal(Enum) (Variables|/Script/ICAN_Card_Game.CardData|GetPlacement (Variables|/Script/ICAN_Card_Game.Card|GetCardDataComp _array_element)) "FLAVOR")
              (bind _result_3 (Math|Integer|IncrementInt (Variables|Default|GetFlavor))
                (:%20%20
                  (Variables|Default|SetFlavor _result_3)))))))))
  (if (Math|Boolean|ORBoolean (== (Variables|Default|GetAmplification) 3) (== (Variables|Default|GetBody) 3) (== (Variables|Default|GetFlavor) 3))
    (return true)
    (else
      (return false))))