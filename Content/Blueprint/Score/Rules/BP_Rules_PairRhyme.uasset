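; BP_Rules_PairRhyme is a card scoring rule that validates whether a set of cards forms a rhyme pair by strength.
; BValidateRule loops over the valid cards and tallies the Idou, Essa and Ultis strengths from each CardDataComp.
; It returns true when any of those tallies is exactly two, so three or more of one strength does not qualify by itself.
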(fn BValidateRule
  (params (Cards :type Array%20of%20Card%20Object%20References))
  (Variables|Default|SetIdou 0)
  (Variables|Default|SetEssa 0)
  (Variables|Default|SetUltis 0)
  (for _array_element Cards
    (Utilities|IsValid _array_element
      (:Is%20Valid
        (Utilities|FlowControl|Sequence
          (:then_0
            (if (Utilities|Enum|Equal(Enum) (Variables|/Script/ICAN_Card_Game.CardData|GetStrength (Variables|/Script/ICAN_Card_Game.Card|GetCardDataComp _array_element)) "IDOU")
              (bind _result (Math|Integer|IncrementInt (Variables|Default|GetIdou))
                (:%20%20
                  (Variables|Default|SetIdou _result)))))
          (:then_1
            (if (Utilities|Enum|Equal(Enum) (Variables|/Script/ICAN_Card_Game.CardData|GetStrength (Variables|/Script/ICAN_Card_Game.Card|GetCardDataComp _array_element)) "ESSA")
              (bind _result_2 (Math|Integer|IncrementInt (Variables|Default|GetEssa))
                (:%20%20
                  (Variables|Default|SetEssa _result_2)))))
          (:then_2
            (if (Utilities|Enum|Equal(Enum) (Variables|/Script/ICAN_Card_Game.CardData|GetStrength (Variables|/Script/ICAN_Card_Game.Card|GetCardDataComp _array_element)) "ULTIS")
              (bind _result_3 (Math|Integer|IncrementInt (Variables|Default|GetUltis))
                (:%20%20
                  (Variables|Default|SetUltis _result_3)))))))))
  (if (Math|Boolean|ORBoolean (== (Variables|Default|GetIdou) 2) (== (Variables|Default|GetEssa) 2) (== (Variables|Default|GetUltis) 2))
    (return true)
    (else
      (return false))))