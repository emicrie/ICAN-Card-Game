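; BP_Rules_Yellendo is a card scoring rule that checks whether a set of cards qualifies as a Yellendo.
; Its validation function loops over the given cards, skips invalid references and counts those whose card data component has ULTIS strength.
; The rule passes only when that count is exactly three, regardless of the other cards in the set.
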(fn BValidateRule
  (params (Cards :type Array%20of%20Card%20Object%20References))
  (Variables|Default|SetUltis 0)
  (for _array_element Cards
    (Utilities|IsValid _array_element
      (:Is%20Valid
        (if (Utilities|Enum|Equal(Enum) (Variables|/Script/ICAN_Card_Game.CardData|GetStrength (Variables|/Script/ICAN_Card_Game.Card|GetCardDataComp _array_element)) "ULTIS")
          (bind _result (Math|Integer|IncrementInt (Variables|Default|GetUltis))
            (:%20%20
              (Variables|Default|SetUltis _result)))))))
  (if (== (Variables|Default|GetUltis) 3)
    (return true)
    (else
      (return false))))