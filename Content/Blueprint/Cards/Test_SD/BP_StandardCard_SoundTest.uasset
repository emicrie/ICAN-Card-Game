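; BP_StandardCard_SoundTest is a card Blueprint used to test FMOD sound playback and global effect parameters.
; Tick runs through a two-second Delay, so it starts a new 2D event instance roughly every two seconds, with no event asset shown assigned.
; When the instance is valid, it sets the global Reverb and Chorus parameters from the Blueprint's matching variables.
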(event EventBeginPlay
  (|CallParentFunction) ; This node is disabled and will not be called.\nDrag off pins to build functionality.
)

(event Collision|EventActorBeginOverlap
  (params (OtherActor :type Actor%20Object%20Reference))
  (|CallParentFunction OtherActor) ; This node is disabled and will not be called.\nDrag off pins to build functionality.
)

(event EventTick
  (params (DeltaSeconds :type Float%20%28single-precision%29))
  (|CallParentFunction DeltaSeconds)
  (Utilities|FlowControl|Delay 2.0)
  (bind _returnvalue (CallFunction|PlayEvent2D))
  (CallFunction|EventInstancePlay _returnvalue)
  (bind _returnvalue_2 (CallFunction|EventInstanceIsValid _returnvalue))
  (if _returnvalue_2
    (CallFunction|SetGlobalParameterbyName "Reverb" (Variables|Default|GetReverb))
    (CallFunction|SetGlobalParameterbyName "Chorus" (Variables|Default|GetChorus))))

(fn ConstructionScript
  (|CallParentFunction))