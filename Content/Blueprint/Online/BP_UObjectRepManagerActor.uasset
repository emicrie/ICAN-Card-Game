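; Replication manager actor for card-game UObjects, meant to share the GameState's deck and players' hands over the network.
; On authority, OnSpawn calls an empty create event, then multicasts the Deck reference into each GameState.
; Deck and hand construction, with registration in RepCardCollectionManager, is present but disconnected, so it never runs.
; Debug helpers print deck capacity after a BeginPlay delay and dump deck cards through an owning-client event.
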(event Custom|OWNCL-DebugCards
  (bind _asbp_game_state (Utilities|Casting|CastToBP_GameState (Game|GetGameState)))
  (Default|DebugDeckCards _asbp_game_state (Variables|/Script/ICAN_Card_Game.ReplicatedCardCollection|GetElements (Variables|/Script/ICAN_Card_Game.CGGameState|GetDeck _asbp_game_state))))

(event Custom|SRV-Create%20ReplicatedObjects)

(event Custom|Display%20Deck%20Size
  (bind _asbp_game_state (Utilities|Casting|CastToBP_GameState (Game|GetGameState)))
  (Utilities|IsValid (Variables|/Script/ICAN_Card_Game.CGGameState|GetDeck _asbp_game_state)
    (:Is%20Valid
      (Development|PrintString (Utilities|String|ToString(Integer) (Variables|/Script/ICAN_Card_Game.ReplicatedCardCollection|GetMaxCapacity (Variables|/Script/ICAN_Card_Game.CGGameState|GetDeck _asbp_game_state)))))
    (:Is%20Not%20Valid
      (Development|PrintString "Deck is not valid"))))

(event Custom|SRV-GetDeckSize
  (bind _asbp_game_state (Utilities|Casting|CastToBP_GameState (Game|GetGameState)))
  (CallFunction|MTC-SetDeckSize (Variables|/Script/ICAN_Card_Game.CGGameState|GetDeck _asbp_game_state)))

(event Custom|MTC-SetDeckSize
  (params (Deck :type Replicated%20Deck%20Object%20Reference))
  (bind _asbp_game_state (Utilities|Casting|CastToBP_GameState (Game|GetGameState)))
  (Variables|/Script/ICAN_Card_Game.CGGameState|SetDeck _asbp_game_state Deck))

(event EventBeginPlay
  (Utilities|Time|SetTimerbyEvent (delegate Custom|Display%20Deck%20Size) 5.0))

(fn ConstructionScript)

(fn OnSpawn
  (Networking|SwitchHasAuthority
    (:Authority
      (CallFunction|SRV-CreateReplicatedObjects)
      (CallFunction|SRV-GetDeckSize))))

(fn DebugCards
  (CallFunction|OWNCL-DebugCards))