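; Online card game state Blueprint that holds a deck reference, with logic that is mostly debug scaffolding.
; A custom event stores an incoming valid deck, while the server-named get and fill events only print debug text, the latter on the Remote branch.
; Random deck filling from the deck's data table and the call to DebugDeckCards, which prints each card's row details, are both disconnected.
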(event Custom|SRV_FillDeck
  (Networking|SwitchHasAuthority
    (:Remote
      (Utilities|IsValid (Variables|Default|GetDeck)
        (:Is%20Valid
          (Development|PrintString "Hello"))))))

(event Custom|SRV_GetDeck
  (Development|PrintString (Utilities|GetDisplayName (Variables|Default|GetDeck)))
  (Development|PrintString (Utilities|String|ToString(Integer) (Variables|Default|GetDeckSize)) true true "(R=1.000000,G=0.000000,B=0.814836,A=1.000000)"))

(event Custom|MTC-%20FROM%20SRV%20-%20SET%20DECK
  (params (Deck :type Replicated%20Deck%20Object%20Reference))
  (Utilities|IsValid Deck
    (:Is%20Valid
      (Development|PrintString "DECK UPDATE VALID")
      (bind _output_get (Variables|Default|SetDeck Deck))
      (Utilities|IsValid _output_get
        (:Is%20Valid
          (Development|PrintString "STILL VALID"))))))

(event EventOnStart)

(event EventTick
  (params (DeltaSeconds :type Float%20%28single-precision%29)))

(fn ConstructionScript)

(fn DebugDeckCards
  (params (CardDatas :type Array%20of%20Replicated%20Card%20Data%20Object%20References))
  (for _array_element CardDatas
    (Development|PrintString (Utilities|String|ToString(Integer) (Variables|/Script/ICAN_Card_Game.ReplicatedCardData|GetID _array_element)))
    (bind _returnvalue (Utilities|GetDataTableRow (Variables|/Script/ICAN_Card_Game.ReplicatedDeck|GetDeckDataTable (Variables|Default|GetDeck)) (Utilities|String|StringToName (Utilities|String|ToString(Integer) (Variables|/Script/ICAN_Card_Game.ReplicatedCardData|GetID _array_element))))
      (:then
        (Development|PrintString (Utilities|String|Append (Utilities|String|Append (Utilities|String|Append (Utilities|String|Append (Utilities|String|Append (Utilities|String|Append (Utilities|String|Append (Utilities|String|Append (Utilities|String|Append "ID:" (Utilities|String|ToString(Integer) (Variables|/Script/ICAN_Card_Game.ReplicatedCardData|GetID _array_element))) " ") (Utilities|String|ToString(Text) (.Name (Utilities|Struct|BreakS_CardStruct _returnvalue)))) " ") (Utilities|String|ToString(Integer) (.Value (Utilities|Struct|BreakS_CardStruct _returnvalue)))) " ") (Utilities|String|EnumtoString (.Strength (Utilities|Struct|BreakS_CardStruct _returnvalue)))) " ") (Utilities|String|EnumtoString (.Placement (Utilities|Struct|BreakS_CardStruct _returnvalue)))) true true "(R=0.000000,G=0.660000,B=1.000000,A=1.000000)" 99.0)))))