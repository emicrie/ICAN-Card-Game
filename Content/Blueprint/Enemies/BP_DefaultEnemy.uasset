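; Default enemy actor that sits at a fixed spot with a spinning Star component and plays a defeat sequence when killed.
; BeginPlay sets its location and Tick rotates the star.
; EnnemyDeath spawns the BossDefeated effect and spell sound, binds itself to a Level Sequence at runtime and plays it, then destroys itself after a short delay.
; A transform-origin override for the sequence is left disconnected.
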(event Custom|EnnemyDeath
  (Niagara|SpawnSystematLocation "/Game/Vefects/BossDefeated.BossDefeated" (+ (Transformation|GetActorLocation) "-100.000000,-50.000000,100.000000"))
  ;[0.2514 0.2753 1] SFX-Spell
  (Class|FMODBlueprintStatics|PlayEvent2D "/Game/FMOD/Events/Spell/Spell.Spell")
  (bind (_outactor _returnvalue) (Sequencer|Player|CreateLevelSequencePlayer (Variables|Default|GetSequencePlayer)))
  (Class|LevelSequenceActor|AddBinding _outactor (|GetSequenceBinding) self false)
  (Sequencer|Player|Play _returnvalue :!class /Script/MovieScene.MovieSceneSequencePlayer)
  (Utilities|FlowControl|Delay 0.6)
  (Actor|DestroyActor))

(event EventTick
  (params (DeltaSeconds :type Float%20%28single-precision%29))
  (Transformation|AddWorldRotation (Variables|Default|GetStar) "0.000000,0.000000,1.000000" false false))

(event EventBeginPlay
  (Transformation|SetActorLocation "110.000000,350.000000,0.000000" false false))

(fn ConstructionScript)