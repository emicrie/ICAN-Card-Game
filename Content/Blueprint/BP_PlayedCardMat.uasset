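; BP_PlayedCardMat is the Blueprint that displays the game's played cards by rebuilding them in the card slots.
; Its update event destroys and clears its current Cards, then loops over the game mode's PlayedCards contents.
; For each element passing a valid-index check (on the element value, not the loop index), it calls the game mode to spawn a card at the matching CardSlotArray location with fixed rotation.
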(event Custom|MTC-UpdateCollectionContent
  (bind _asbp_card_game_mode (Utilities|Casting|CastToBP_CardGameMode (Game|GetGameMode)))
  (CallFunction|EmptyCards)
  (for (_array_element _array_index) (Variables|/Script/ICAN_Card_Game.CardCollection|GetContents (Variables|/Script/ICAN_Card_Game.CardGameMode|GetPlayedCards _asbp_card_game_mode))
    (if (Utilities|Array|IsValidIndex (Variables|/Script/ICAN_Card_Game.CardCollection|GetContents (Variables|/Script/ICAN_Card_Game.CardGameMode|GetPlayedCards _asbp_card_game_mode)) _array_element)
      (bind _asbp_card_game_mode_2 (Utilities|Casting|CastToBP_CardGameMode (Game|GetGameMode)))
      (Default|MTC-SpawnNewCardinPlayedSlots _asbp_card_game_mode (Math|Transform|MakeTransform (Transformation|GetWorldLocation (Utilities|Array|Get(acopy) (Variables|/Game/Blueprint/Online/BP_CardGameMode.BP_CardGameMode_C|GetCardSlotArray _asbp_card_game_mode_2) _array_index)) "-90.000000,0.000000,0.000000") (Variables|/Script/ICAN_Card_Game.CardGameMode|GetPlayedCards _asbp_card_game_mode) _array_element _array_index))))

(fn ConstructionScript)

(fn EmptyCards
  (bind _cards (Variables|Default|GetCards))
  (for _array_element _cards
    (Utilities|IsValid _array_element
      (:Is%20Valid
        (Actor|DestroyActor _array_element))))
  (Utilities|Array|Clear _cards))